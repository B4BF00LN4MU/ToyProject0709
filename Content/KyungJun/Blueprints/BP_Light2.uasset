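; BP_Light2 is a light actor whose RectLight responds to a Switch's overlap state.
; On BeginPlay it prints its name, hides the light and binds to the Switch's toggle dispatcher, with EventSwitchOverlap setting IsPlay.
; Tick polls IsPlay, showing the light after a short Delay when true and hiding it when false.
; Disconnected nodes hold unused logic for stepping a relative location along X and Z.
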(event `self.ReceiveBeginPlay`
  (`KismetSystemLibrary.PrintString` (`KismetSystemLibrary.GetDisplayName` self) true true (struct :`G` 0.66 :`B` 1.0 :`A` 1.0) 60.0)
  (`SceneComponent.SetVisibility` (`self.RectLight`) false false)
  (add `/Game/KyungJun/Blueprints/BP_ToggleSwitch.EventDispatcher_EventToggle` (`self.Switch`) (`|CreateDelegate` :!event `EventSwitchOverlap`)))

(event `self.ReceiveTick`
  (params (DeltaSeconds :type "Float (single-precision)"))
  (bind _rectlight (`self.RectLight`))
  (if (`self.IsPlay`)
    (`KismetSystemLibrary.Delay` 2.0)
    (`SceneComponent.SetVisibility` _rectlight true false)
    (else
      (`SceneComponent.SetVisibility` _rectlight false false))))

(fn `EventSwitchOverlap`
  (params (IsBegin :type Boolean))
  (set `self.IsPlay` IsBegin))

(fn `UserConstructionScript`)