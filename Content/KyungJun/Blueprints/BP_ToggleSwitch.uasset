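; BP_ToggleSwitch is a switch actor that flips an on/off state and shows it through its mesh material.
; DoToggleSwitch inverts IsOn, swaps the StaticMesh material to match, then fires the EventToggle dispatcher with the new state.
; Its overlap and line-trace click handlers only forward to the parent class, and nothing in this file calls DoToggleSwitch.
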(fn `DoToggleSwitch`
  (bind _staticmesh (`self.StaticMesh`))
  (bind _output_get (set `self.IsOn` (not (`self.IsOn`))))
  (if _output_get
    (`PrimitiveComponent.SetMaterial` _staticmesh 0 "/Engine/MapTemplates/Materials/BasicAsset01.BasicAsset01")
    (else
      (`PrimitiveComponent.SetMaterial` _staticmesh 0 "/Engine/BasicShapes/BasicShapeMaterial.BasicShapeMaterial")))
  (`self.EventDispatcher_EventToggle` (`self.IsOn`)))

(fn `OnBeginOverlap`
  (`parent.OnBeginOverlap`))

(fn `OnEndOverlap`
  (`parent.OnEndOverlap`))

(fn `OnLineTraceClick`
  (`parent.OnLineTraceClick`))

(fn `UserConstructionScript`)