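; BP_MoveRect1 is an actor that moves its static mesh around a square path in the local XZ plane while switched on.
; BeginPlay prints the actor's name and binds to the toggle dispatcher of a referenced Switch, with EventSwitchOverlap setting IsPlay from the overlap state.
; While IsPlay is true, Tick cycles a Right, Up, Left, Down state machine, stepping a fixed amount per frame, so speed depends on frame rate.
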(event `self.ReceiveBeginPlay`
  (`KismetSystemLibrary.PrintString` (`KismetSystemLibrary.GetDisplayName` self) true true (struct :`G` 0.66 :`B` 1.0 :`A` 1.0) 60.0)
  (add `/Game/KyungJun/Blueprints/BP_ToggleSwitch.EventDispatcher_EventToggle` (`self.Switch`) (`|CreateDelegate` :!event `EventSwitchOverlap`)))

(event `self.ReceiveTick`
  (params (DeltaSeconds :type "Float (single-precision)"))
  (if (`self.IsPlay`)
    (switch `/Game/KyungJun/Blueprints/EN_MoveType` (`self.MoveType`)
      (:`NewEnumerator0`
        ;[1 1 1] 오른쪽으로 이동
        (set `self.X에위치` (+ (`self.X에위치`) 1.0))
        (`SceneComponent.K2_SetRelativeLocation` (`self.StaticMesh`) (`KismetMathLibrary.MakeVector` (`self.X에위치`)) false false)
        (if (> (`self.X에위치`) 200.0)
          (set `self.MoveType` "NewEnumerator1")))
      (:`NewEnumerator1`
        ;[1 1 1] 위쪽으로 이동
        (set `self.Z에위치` (+ (`self.Z에위치`) 1.0))
        (`SceneComponent.K2_SetRelativeLocation` (`self.StaticMesh`) (`KismetMathLibrary.MakeVector` (`self.X에위치`) 0.0 (`self.Z에위치`)) false false)
        (if (> (`self.Z에위치`) 200.0)
          (set `self.MoveType` "NewEnumerator2")))
      (:`NewEnumerator2`
        ;[1 1 1] 왼쪽으로 이동
        (set `self.X에위치` (+ (`self.X에위치`) -1.0))
        (`SceneComponent.K2_SetRelativeLocation` (`self.StaticMesh`) (`KismetMathLibrary.MakeVector` (`self.X에위치`) 0.0 (`self.Z에위치`)) false false)
        (if (< (`self.X에위치`) 0.0)
          (set `self.MoveType` "NewEnumerator3")))
      (:`NewEnumerator3`
        ;[1 1 1] 아래쪽으로 이동
        (set `self.Z에위치` (+ (`self.Z에위치`) -1.0))
        (`SceneComponent.K2_SetRelativeLocation` (`self.StaticMesh`) (`KismetMathLibrary.MakeVector` 0.0 0.0 (`self.Z에위치`)) false false)
        (if (< (`self.Z에위치`) 0.0)
          (set `self.MoveType` "NewEnumerator0"))))))

(fn `EventSwitchOverlap`
  (params (IsBegin :type Boolean))
  (set `self.IsPlay` IsBegin))

(fn `UserConstructionScript`)