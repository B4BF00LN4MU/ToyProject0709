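; BP_MoveLeftRight is an actor whose static mesh slides back and forth along relative X while an overlap switch is active.
; On BeginPlay it binds EventSwitchOverlap to the overlap dispatcher of the referenced 조인성 object, which sets IsPlay from the begin/end state.
; While IsPlay is true, Tick steps the position by a fixed per-frame amount, independent of delta time, reversing direction at each limit.
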(event `self.ReceiveBeginPlay`
  (add `/Game/KyungJun/Blueprints/BP_Switch.EventDispatcher_Overlap` (`self.조인성`) (`|CreateDelegate` :!event `EventSwitchOverlap`)))

(event `self.ReceiveTick`
  (params (DeltaSeconds :type "Float (single-precision)"))
  (if (`self.IsPlay`)
    (if (`self.오른쪽으로이동하니?`)
      ;[1 1 1] 오른쪽으로 이동
      (set `self.X에위치` (+ (`self.X에위치`) 1.0))
      (`SceneComponent.K2_SetRelativeLocation` (`self.StaticMesh`) (`KismetMathLibrary.MakeVector` (`self.X에위치`)) false false)
      (if (> (`self.X에위치`) 200.0)
        (set `self.오른쪽으로이동하니?` false))
      (else
        ;[1 1 1] 왼쪽으로 이동
        (set `self.X에위치` (+ (`self.X에위치`) -1.0))
        (`SceneComponent.K2_SetRelativeLocation` (`self.StaticMesh`) (`KismetMathLibrary.MakeVector` (`self.X에위치`)) false false)
        (if (< (`self.X에위치`) 0.0)
          (set `self.오른쪽으로이동하니?` true))))))

(fn `EventSwitchOverlap`
  (params (IsBegin :type Boolean))
  (set `self.IsPlay` IsBegin)
  (return))

(fn `UserConstructionScript`)