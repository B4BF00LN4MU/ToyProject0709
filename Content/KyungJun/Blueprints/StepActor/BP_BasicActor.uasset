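; BP_BasicActor is a base actor for a step-driven content flow, with empty start-step and line-trace-click hooks.
; On BeginPlay it binds to BP_StepGameState's content-state change dispatcher, calling EventStartStep when the state matches MyStep and OnLineTraceClick otherwise.
; EventEndStep advances the game state to NextStep.
; The construction script writes both step names to a text render component as a label.
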(event `self.ReceiveBeginPlay`
  (`self.BindGameState`))

(fn `BindGameState`
  (bind _asbp_step_game_state (cast `/Game/KyungJun/GameMode/BP_StepGameState` (`GameplayStatics.GetGameState`)))
  (add `/Game/KyungJun/GameMode/BP_StepGameState.EventDispatcher_ChangeContentState` _asbp_step_game_state (`|CreateDelegate` :!event `EventChangeContentState`)))

(fn `EventChangeContentState`
  (params (ContentState :type "/Game/KyungJun/Blueprints/EN_ContentState Enum" :default "NewEnumerator0"))
  (if (== ContentState (`self.MyStep`))
    (`self.EventStartStep`)
    (else
      (`self.On Line Trace Click`))))

(fn `EventEndStep`
  (bind _asbp_step_game_state (cast `/Game/KyungJun/GameMode/BP_StepGameState` (`GameplayStatics.GetGameState`)))
  (`/Game/KyungJun/GameMode/BP_StepGameState.ChangeContentState` _asbp_step_game_state (`self.NextStep`)))

(fn `EventStartStep`)

(fn `On Line Trace Click`)

(fn `UserConstructionScript`
  (`TextRenderComponent.K2_SetText` (`self.TextRender`) (`KismetTextLibrary.Conv_StringToText` (`KismetStringLibrary.Concat_StrStr` (`|GetEnumeratorNameAsString` (`self.MyStep`)) " " (`|GetEnumeratorNameAsString` (`self.NextStep`))))))