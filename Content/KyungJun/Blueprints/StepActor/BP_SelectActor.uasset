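; A selectable step actor that the player picks with a line-trace click to complete its step.
; It starts hidden and without collision; starting the step enables the box collision and select tracing on the BP_ToyPerson player pawn.
; Overlap begin and end show and hide a decal highlight.
; A click turns off tracing, collision and decal, then ends the step.
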(event `self.ReceiveBeginPlay`
  (`parent.ReceiveBeginPlay`)
  (`SceneComponent.SetVisibility` (`self.Decal`) false false)
  (`PrimitiveComponent.SetCollisionEnabled` (`self.Box`) "NoCollision"))

(fn `EventStartStep`
  (`parent.EventStartStep`)
  (bind _asbp_toy_person (cast `/Game/KyungJun/Blueprints/BP_ToyPerson` (`GameplayStatics.GetPlayerPawn` 0)))
  (`/Game/KyungJun/Blueprints/BP_ToyPerson.SetSelectLineTrace` _asbp_toy_person true)
  (`PrimitiveComponent.SetCollisionEnabled` (`self.Box`) "QueryAndPhysics"))

(fn `OnBeginOverlap`
  (`SceneComponent.SetVisibility` (`self.Decal`) true false))

(fn `OnEndOverlap`
  (`SceneComponent.SetVisibility` (`self.Decal`) false false))

(fn `OnLineTraceClick`
  (bind _asbp_toy_person (cast `/Game/KyungJun/Blueprints/BP_ToyPerson` (`GameplayStatics.GetPlayerPawn` 0)))
  (`/Game/KyungJun/Blueprints/BP_ToyPerson.SetSelectLineTrace` _asbp_toy_person false)
  (`PrimitiveComponent.SetCollisionEnabled` (`self.Box`) "NoCollision")
  (`SceneComponent.SetVisibility` (`self.Decal`) false false)
  (`self.EventEndStep`))

(fn `UserConstructionScript`
  (`parent.UserConstructionScript`))