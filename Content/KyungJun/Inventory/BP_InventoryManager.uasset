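; BP_InventoryManager is an early-stage inventory manager actor that holds an Inventory array with a size limit.
; AddItem checks the length against MaxInventorySize, then replaces the array with just the new item rather than appending.
; UpdateInventory loops over the array, overwriting it with each single element, and has an unconnected MaxInventorySize setter.
; The event graph and construction script are empty.
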(fn `AddItem`
  (params (NewItem :type "/Game/KyungJun/Inventory/BP_InventoryItem Object Reference"))
  (if (< (`KismetArrayLibrary.Array_Length` (`self.Inventory`)) (`self.MaxInventorySize`))
    (set `self.Inventory` (`|MakeArray` NewItem))))

(fn `UpdateInventory`
  (for (_array_element _array_index) (`self.Inventory`)
    (set `self.Inventory` (`|MakeArray` _array_element))))

(fn `UserConstructionScript`)